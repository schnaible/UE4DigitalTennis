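; BP_BallMenu is a Pong-style ball, likely for the menu background, that launches diagonally on BeginPlay using physics velocity.
; On overlap, casts identify what it hit: horizontal boundaries flip X, while paddles and the left goal flip Y.
; Paddles also randomize X; only the right paddle adds its own velocity.
; The goal just bounces the ball without scoring, and each handled hit plays a collision sound.
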(event EventBeginPlay
  (Physics|SetPhysicsLinearVelocity (Variables|Default|GetStaticMesh) "2000.000000,2000.000000, 0" false "None"))

(event Collision|EventActorBeginOverlap
  (params (OtherActor :type Actor%20Object%20Reference))
  (Utilities|Casting|CastToBP_HorizontalBoundary OtherActor
    (:then
      (bind _returnvalue (Physics|GetPhysicsLinearVelocity (Variables|Default|GetStaticMesh) "None"))
      (Physics|SetPhysicsLinearVelocity (Variables|Default|GetStaticMesh) (Math|Vector|MakeVector (* (.X (Math|Vector|BreakVector _returnvalue)) -1.0) (.Y (Math|Vector|BreakVector _returnvalue)) (.Z (Math|Vector|BreakVector _returnvalue))) false "None")
      (Audio|PlaySoundatLocation "/Game/Audio/S_ballCollision.S_ballCollision" "0, 0, 0" "0, 0, 0" 1.0 1.0 0.0 0 0 0))
    (:CastFailed
      (bind _asbp_pattle_pawn_right (Utilities|Casting|CastToBP_Pattle_Pawn_Right OtherActor)
        (:then
          (bind _returnvalue_2 (Physics|GetPhysicsLinearVelocity (Variables|/Game/Blueprints/BP_Pattle_Pawn_Right.BP_Pattle_Pawn_Right_C|GetPaddle_Mesh _asbp_pattle_pawn_right) "None"))
          (bind _returnvalue_3 (Physics|GetPhysicsLinearVelocity (Variables|Default|GetStaticMesh) "None"))
          (Physics|SetPhysicsLinearVelocity (Variables|Default|GetStaticMesh) (Math|Vector|MakeVector (+ (.X (Math|Vector|BreakVector _returnvalue_2)) (Math|Random|RandomFloatinRange -1e+03 1e+03)) (* (.Y (Math|Vector|BreakVector _returnvalue_3)) -1.0) (.Z (Math|Vector|BreakVector _returnvalue_3))) false "None")
          (Audio|PlaySoundatLocation "/Game/Audio/S_ballCollision.S_ballCollision" "0, 0, 0" "0, 0, 0" 1.0 1.0 0.0 0 0 0))
        (:CastFailed
          (bind _asbp_paddle_l (Utilities|Casting|CastToBP_Paddle_L OtherActor)
            (:then
              (Physics|GetPhysicsLinearVelocity (Variables|/Game/Blueprints/BP_Paddle_L.BP_Paddle_L_C|GetStaticMesh _asbp_paddle_l) "None")
              (bind _returnvalue_4 (Physics|GetPhysicsLinearVelocity (Variables|Default|GetStaticMesh) "None"))
              (Physics|SetPhysicsLinearVelocity (Variables|Default|GetStaticMesh) (Math|Vector|MakeVector (+ (.X (Math|Vector|BreakVector "0, 0, 0")) (Math|Random|RandomFloatinRange -1e+03 1e+03)) (* (.Y (Math|Vector|BreakVector _returnvalue_4)) -1.0) (.Z (Math|Vector|BreakVector _returnvalue_4))) false "None")
              (Audio|PlaySoundatLocation "/Game/Audio/S_ballCollision.S_ballCollision" "0, 0, 0" "0, 0, 0" 1.0 1.0 0.0 0 0 0))
            (:CastFailed
              (Utilities|Casting|CastToBP_L_Goal OtherActor)
              (bind _returnvalue_5 (Physics|GetPhysicsLinearVelocity (Variables|Default|GetStaticMesh) "None"))
              (Physics|SetPhysicsLinearVelocity (Variables|Default|GetStaticMesh) (Math|Vector|MakeVector (.X (Math|Vector|BreakVector _returnvalue_5)) (* (.Y (Math|Vector|BreakVector _returnvalue_5)) -1.0) (.Z (Math|Vector|BreakVector _returnvalue_5))) false "None")
              (Audio|PlaySoundatLocation "/Game/Audio/S_ballCollision.S_ballCollision" "0, 0, 0" "0, 0, 0" 1.0 1.0 0.0 0 0 0))))))))

(fn ConstructionScript)